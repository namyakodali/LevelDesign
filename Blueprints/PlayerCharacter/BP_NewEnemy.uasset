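; Laser enemy that hurts and knocks back the player on contact, and is destroyed when the player overlaps its head zone.
; A looping timer with a random start delay calls Lasers, which randomly switches the three cylinders' visibility and collision, plus both trigger zones' collision, on or off together.
; Box overlap decreases player health and launches them horizontally away from the box, scaled by Launch.
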(event OnComponentBeginOverlap(HeadZone)
  (params (OverlappedComponent :type Primitive%20Component%20Object%20Reference) (OtherActor :type Actor%20Object%20Reference) (OtherComp :type Primitive%20Component%20Object%20Reference) (OtherBodyIndex :type Integer) (bFromSweep :type Boolean) (SweepResult :type Hit%20Result%20Structure%20%28by%20ref%29))
  (Utilities|Casting|CastToBP_LearningKit_PlayerCharacter OtherActor)
  (Actor|DestroyActor))

(event OnComponentBeginOverlap(Box)
  (params (OverlappedComponent :type Primitive%20Component%20Object%20Reference) (OtherActor :type Actor%20Object%20Reference) (OtherComp :type Primitive%20Component%20Object%20Reference) (OtherBodyIndex :type Integer) (bFromSweep :type Boolean) (SweepResult :type Hit%20Result%20Structure%20%28by%20ref%29))
  (bind _asbp_learning_kit_player_character (Utilities|Casting|CastToBP_LearningKit_PlayerCharacter OtherActor))
  (Default|DecreaseHealth _asbp_learning_kit_player_character)
  (Character|LaunchCharacter _asbp_learning_kit_player_character (* (Math|Vector|MakeVector (.x (Math|Vector|Normalize (Math|Vector|MakeVector (.x (Math|Vector|GetUnitDirection(Vector) (Transformation|GetWorldLocation (Variables|Default|GetBox)) (Transformation|GetActorLocation _asbp_learning_kit_player_character))) (.y (Math|Vector|GetUnitDirection(Vector) (Transformation|GetWorldLocation (Variables|Default|GetBox)) (Transformation|GetActorLocation _asbp_learning_kit_player_character))) 0.0))) (.y (Math|Vector|Normalize (Math|Vector|MakeVector (.x (Math|Vector|GetUnitDirection(Vector) (Transformation|GetWorldLocation (Variables|Default|GetBox)) (Transformation|GetActorLocation _asbp_learning_kit_player_character))) (.y (Math|Vector|GetUnitDirection(Vector) (Transformation|GetWorldLocation (Variables|Default|GetBox)) (Transformation|GetActorLocation _asbp_learning_kit_player_character))) 0.0))) 0.0) (Variables|Default|GetLaunch)) false false))

(event EventBeginPlay
  (Utilities|Time|SetTimerbyFunctionName 0 "Lasers" 0.5 true (Math|Random|RandomFloatinRange 0.0 2.0)))

(event Collision|EventActorBeginOverlap
  (params (OtherActor :type Actor%20Object%20Reference)))

(fn ConstructionScript)

(fn Lasers
  (if (< (Math|Random|RandomFloatinRange 0.0 1e+01) 5.0)
    (Utilities|FlowControl|Sequence
      (:then_0
        (Rendering|SetVisibility (Variables|Default|GetCylinder) false false)
        (Collision|SetCollisionEnabled (Variables|Default|GetCylinder) "NoCollision"))
      (:then_1
        (Rendering|SetVisibility (Variables|Default|GetCylinder1) false false)
        (Collision|SetCollisionEnabled (Variables|Default|GetCylinder1) "NoCollision"))
      (:then_2
        (Rendering|SetVisibility (Variables|Default|GetCylinder2) false false)
        (Collision|SetCollisionEnabled (Variables|Default|GetCylinder2) "NoCollision"))
      (:then_3
        (Collision|SetCollisionEnabled (Variables|Default|GetBox) "NoCollision"))
      (:then_4
        (Collision|SetCollisionEnabled (Variables|Default|GetHeadZone) "NoCollision")))
    (else
      (Utilities|FlowControl|Sequence
        (:then_0
          (Rendering|SetVisibility (Variables|Default|GetCylinder) true false)
          (Collision|SetCollisionEnabled (Variables|Default|GetCylinder) "QueryAndPhysics"))
        (:then_1
          (Rendering|SetVisibility (Variables|Default|GetCylinder1) true false)
          (Collision|SetCollisionEnabled (Variables|Default|GetCylinder1) "QueryAndPhysics"))
        (:then_2
          (Rendering|SetVisibility (Variables|Default|GetCylinder2) true false)
          (Collision|SetCollisionEnabled (Variables|Default|GetCylinder2) "QueryAndPhysics"))
        (:then_3
          (Collision|SetCollisionEnabled (Variables|Default|GetBox) "QueryAndPhysics"))
        (:then_4
          (Collision|SetCollisionEnabled (Variables|Default|GetHeadZone) "QueryAndPhysics"))))))