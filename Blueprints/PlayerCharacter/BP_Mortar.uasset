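; BP_Mortar is a hazard actor that repeatedly launches projectiles and is destroyed when the learning-kit player character overlaps its HeadZone.
; BeginPlay starts a looping timer with a random initial delay that calls ShootProjectile by name.
; ShootProjectile spawns a BP_Projectile above the mortar with slight horizontal position jitter and a random yaw.
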(event OnComponentBeginOverlap(HeadZone)
  (params (OverlappedComponent :type Primitive%20Component%20Object%20Reference) (OtherActor :type Actor%20Object%20Reference) (OtherComp :type Primitive%20Component%20Object%20Reference) (OtherBodyIndex :type Integer) (bFromSweep :type Boolean) (SweepResult :type Hit%20Result%20Structure%20%28by%20ref%29))
  (Utilities|Casting|CastToBP_LearningKit_PlayerCharacter OtherActor)
  (Actor|DestroyActor))

(event EventBeginPlay
  (Utilities|Time|SetTimerbyFunctionName 0 "ShootProjectile" 0.5 true (Math|Random|RandomFloatinRange 0.0 2.0)))

(event Collision|EventActorBeginOverlap
  (params (OtherActor :type Actor%20Object%20Reference)))

(event EventTick
  (params (DeltaSeconds :type Float%20%28single-precision%29)))

(fn ConstructionScript)

(fn ShootProjectile
  (bind _returnvalue (Transformation|GetActorLocation))
  (Game|SpawnActorfromClass "/Game/LearningKit_Games/Blueprints/PlayerCharacter/BP_Projectile.BP_Projectile_C" (Math|Transform|MakeTransform (Math|Vector|MakeVector (Math|Random|RandomFloatinRange (- (.x _returnvalue) 2e+01) (+ (.x _returnvalue) 2e+01)) (Math|Random|RandomFloatinRange (- (.y _returnvalue) 2e+01) (+ (.y _returnvalue) 2e+01)) (+ (.z _returnvalue) 3.5e+02)) (Math|Rotator|MakeRotator 0.0 0.0 (Math|Random|RandomFloatinRange -2e+02 2e+02)) "1.000000,1.000000,1.000000") "Undefined" "MultiplyWithRoot" 0 0))